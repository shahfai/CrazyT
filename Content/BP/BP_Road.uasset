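; BP_Road is a road segment for an endless driving game that extends the road when the SportsCar_Pawn overlaps its Box, via VehicleAdvGameMode.
; The construction script builds candidate spawn points from arrows in two rows at each LinePos lane offset.
; It then attaches one child actor at a random point, choosing between a rare branch and two equally likely ones.
; GetAttachPoint exposes the Arrow's world transform.
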(event `self.Box.OnComponentBeginOverlap`
  (params (OverlappedComponent :type "PrimitiveComponent Object Reference") (OtherActor :type "Actor Object Reference") (OtherComp :type "PrimitiveComponent Object Reference") (OtherBodyIndex :type Integer) (bFromSweep :type Boolean) (SweepResult :type "HitResult Structure (by ref)"))
  (cast `/Game/VehicleTemplate/Blueprints/SportsCar/SportsCar_Pawn` OtherActor)
  (bind _asvehicle_adv_game_mode (cast `/Game/VehicleTemplate/Blueprints/VehicleAdvGameMode` (`GameplayStatics.GetGameMode`)))
  (`/Game/VehicleTemplate/Blueprints/VehicleAdvGameMode.ExtendRoad` _asvehicle_adv_game_mode))

(fn `GetAttachPoint`
  (returns (ReturnValue :type "Transform Structure"))
  (return (`SceneComponent.K2_GetComponentToWorld` (`self.Arrow`))))

(fn `SetArrowSpawn`
  (for _array_element (`self.LinePos`)
    (for _index (range 2)
      (bind _returnvalue (`AddComponent|NODE_AddArrowComponent-0` :`RelativeTransform` (`KismetMathLibrary.MakeTransform` (`KismetMathLibrary.MakeVector` (* _index 650.0) _array_element))))
      (`KismetArrayLibrary.Array_Add` (`self.SpawnArrow`) (`SceneComponent.K2_GetComponentToWorld` _returnvalue)))))

(fn `SpawnBlockers`
  (locals (RandomSpawnArrow :type "Array of Transform Structure"))
  (bind _spawnarrow (`self.SpawnArrow`))
  (bind _returnvalue (`KismetMathLibrary.MakeRelativeTransform` (`|GetArrayItem` (`local.RandomSpawnArrow`) (`.OutIndex` (`KismetArrayLibrary.Array_Random` _spawnarrow))) (`self.GetTransform`)))
  (bind _output_get (set `local.RandomSpawnArrow` _spawnarrow))
  (`KismetArrayLibrary.Array_Shuffle` _output_get)
  (if (<= (`KismetMathLibrary.RandomFloatInRange` 0.0 1.0) 0.025)
    (`AddComponent|NODE_AddChildActorComponent-2` :`RelativeTransform` _returnvalue)
    (else
      (switch `int` (`KismetMathLibrary.RandomIntegerInRange` 0 1)
        (:`0`
          (`AddComponent|NODE_AddChildActorComponent-0` :`RelativeTransform` _returnvalue))
        (:`1`
          (`AddComponent|NODE_AddChildActorComponent-1` :`RelativeTransform` _returnvalue))))))

(fn `UserConstructionScript`
  (`self.SetArrowSpawn`)
  (`self.SpawnBlockers`))